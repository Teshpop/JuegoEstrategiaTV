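; Actor component that tracks whether its owning actor sits in a valid spot for object placement.
; On BeginPlay it binds the owner's begin and end overlap events and runs an initial check.
; Each check sets IsPlacementValid to true only when the owner overlaps no other actors.
; The branch on that result is an empty placeholder for later UI feedback.
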(event Custom|OverlapStatusChange
  (params (OverlappedActor :type Actor%20Object%20Reference) (OtherActor :type Actor%20Object%20Reference))
  (CallFunction|UpdateState))

(event EventBeginPlay
  (bind _returnvalue (Components|GetOwner))
  (Collision|BindEventtoOnActorBeginOverlap _returnvalue (delegate Custom|OverlapStatusChange))
  (Collision|BindEventtoOnActorEndOverlap _returnvalue (delegate Custom|OverlapStatusChange))
  (CallFunction|UpdateState))

(fn UpdateState
  (bind _output_get (Variables|Default|SetIsPlacementValid (== (Utilities|Array|Length (Collision|GetOverlappingActors (Components|GetOwner) "/Script/Engine.Actor" :!class /Script/Engine.Actor)) 0)))
  ;[0 0.5288 1] UI change for later
  (if _output_get
    _))