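; Player action that selects a tile on the grid, toggling it off when the same tile is chosen again.
; ExecuteAction moves the selection state on BPGrid from the previous tile to the new index and stores it in PlayerActions.SelectedTile.
; An off-grid sentinel index means no selection, and destroying the action runs ExecuteAction with it to clear the current selection.
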(event EventDestroyed
  (CallFunction|ExecuteAction (Utilities|Struct|MakeIntPoint -999 -999)))

(fn ConstructionScript
  (|CallParentFunction))

(fn ExecuteAction
  (params (Index :type Int%20Point%20Structure))
  (bind _playeractions (Variables|Default|GetPlayerActions))
  (bind _playeractions_2 (Variables|Default|GetPlayerActions))
  (bind _playeractions_3 (Variables|Default|GetPlayerActions))
  (if (!= (Variables|/Game/_Renato/Revamp_Core/Player/BP_PlayerActions.BP_PlayerActions_C|GetSelectedTile (Variables|Default|GetPlayerActions)) Index)
    (Default|RemoveStatefromTile (Variables|/Game/_Renato/Revamp_Core/Player/BP_PlayerActions.BP_PlayerActions_C|GetBP_Grid _playeractions_3) (Variables|/Game/_Renato/Revamp_Core/Player/BP_PlayerActions.BP_PlayerActions_C|GetSelectedTile _playeractions_3) "NewEnumerator2")
    (Variables|/Game/_Renato/Revamp_Core/Player/BP_PlayerActions.BP_PlayerActions_C|SetSelectedTile (Variables|Default|GetPlayerActions) Index)
    (Default|AddStatetoTile (Variables|/Game/_Renato/Revamp_Core/Player/BP_PlayerActions.BP_PlayerActions_C|GetBP_Grid _playeractions) (Variables|/Game/_Renato/Revamp_Core/Player/BP_PlayerActions.BP_PlayerActions_C|GetSelectedTile _playeractions) "NewEnumerator2")
    (else
      (Default|RemoveStatefromTile (Variables|/Game/_Renato/Revamp_Core/Player/BP_PlayerActions.BP_PlayerActions_C|GetBP_Grid _playeractions_2) (Variables|/Game/_Renato/Revamp_Core/Player/BP_PlayerActions.BP_PlayerActions_C|GetSelectedTile _playeractions_2) "NewEnumerator2")
      (Variables|/Game/_Renato/Revamp_Core/Player/BP_PlayerActions.BP_PlayerActions_C|SetSelectedTile (Variables|Default|GetPlayerActions) (Utilities|Struct|MakeIntPoint -999 -999)))))