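; Player action that places sword units on the grid map when executed on a tile index.
; While adding is enabled, it checks through the PlayerActions grid that the tile is walkable and that the sword troop count is nonzero.
; It spawns BP_Sword at the tile's transform with a height offset, then decrements the count.
; Registration with the combat manager is unconnected, and UnitType is unused.
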(event EventBeginPlay
  (|CallParentFunction) ; This node is disabled and will not be called.\nDrag off pins to build functionality.
)

(event Collision|EventActorBeginOverlap
  (params (OtherActor :type Actor%20Object%20Reference))
  (|CallParentFunction OtherActor) ; This node is disabled and will not be called.\nDrag off pins to build functionality.
)

(event EventTick
  (params (DeltaSeconds :type Float%20%28single-precision%29))
  (|CallParentFunction DeltaSeconds) ; This node is disabled and will not be called.\nDrag off pins to build functionality.
)

(fn ConstructionScript
  (|CallParentFunction))

(fn ExecuteAction
  (params (Index :type Int%20Point%20Structure))
  (bind _playeractions (Variables|Default|GetPlayerActions))
  (bind _bp_grid (Variables|/Game/_Renato/Revamp_Core/Player/BP_PlayerActions.BP_PlayerActions_C|GetBP_Grid _playeractions))
  (bind _gridtiles (Variables|/Game/_Renato/Revamp_Core/Grid/Blueprints/BP_GenerateGrid.BP_GenerateGrid_C|GetGridTiles _bp_grid))
  (bind _value (Utilities|Map|Find _gridtiles Index))
  (bind _transform (Utilities|Struct|BreakS_TileData _value))
  (bind (_location _rotation) (Math|Transform|BreakTransform _transform))
  (if (Variables|Default|GetIsAddingUnit?)
    (if (and (Default|IsTileWalkable (Variables|/Game/_Renato/Revamp_Core/Player/BP_PlayerActions.BP_PlayerActions_C|GetBP_Grid (Variables|Default|GetPlayerActions)) Index) (!= (Variables|Default|GetSwordTroopCount) 0))
      (Game|SpawnActorfromClass "/Game/Tello/Character/BP_Sword.BP_Sword_C" (Math|Transform|MakeTransform (+ _location (Math|Vector|MakeVector 1.0 1.0 (Variables|/Game/_Renato/Revamp_Core/Grid/Blueprints/BP_GenerateGrid.BP_GenerateGrid_C|GetHeightOffset _bp_grid))) _rotation) "AlwaysSpawn" "MultiplyWithRoot" 0 0)
      (Math|Integer|DecrementInt (Variables|Default|GetSwordTroopCount)))))