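; Player action that changes the type of a tile on the grid at a given index.
; On execute, it validates the index against the player actions' grid and looks up that tile's data.
; It re-adds the tile with the action's NewTileType, keeping its index, transform and state.
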(fn ConstructionScript
  (|CallParentFunction))

(fn ExecuteAction
  (params (Index :type Int%20Point%20Structure))
  (if (Default|IsIndexValid (Variables|/Game/_Renato/Revamp_Core/Player/BP_PlayerActions.BP_PlayerActions_C|GetBP_Grid (Variables|Default|GetPlayerActions)) Index)
    (LocalVariables|SetData (.Value (Utilities|Map|Find (Variables|/Game/_Renato/Revamp_Core/Grid/Blueprints/BP_GenerateGrid.BP_GenerateGrid_C|GetGridTiles (Variables|/Game/_Renato/Revamp_Core/Player/BP_PlayerActions.BP_PlayerActions_C|GetBP_Grid (Variables|Default|GetPlayerActions))) Index)))
    (Default|AddGridTile (Variables|/Game/_Renato/Revamp_Core/Player/BP_PlayerActions.BP_PlayerActions_C|GetBP_Grid (Variables|Default|GetPlayerActions)) (Utilities|Struct|MakeS_TileData (.Index (Utilities|Struct|BreakS_TileData (LocalVariables|GetData))) (Variables|Default|GetNewTileType) (.Transform (Utilities|Struct|BreakS_TileData (LocalVariables|GetData))) (.TileState (Utilities|Struct|BreakS_TileData (LocalVariables|GetData)))))))