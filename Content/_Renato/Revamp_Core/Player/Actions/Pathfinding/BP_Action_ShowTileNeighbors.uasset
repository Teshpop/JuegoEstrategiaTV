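; A grid player action that highlights the walkable neighbors of a given tile, likely as a pathfinding aid.
; Executing it clears one tile state across the grid, asks the grid pathfinding component for valid non-diagonal neighbors, and adds a highlight state to each.
; On destruction it runs with an off-grid sentinel index, which clears the highlights.
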(event EventDestroyed
  (CallFunction|ExecuteAction (Utilities|Struct|MakeIntPoint -999 -999)))

(fn ConstructionScript
  (|CallParentFunction))

(fn ExecuteAction
  (params (Index :type Int%20Point%20Structure))
  (Default|ClearAllTIleStates (Variables|/Game/_Renato/Revamp_Core/Player/BP_PlayerActions.BP_PlayerActions_C|GetBP_Grid (Variables|Default|GetPlayerActions)) "NewEnumerator3")
  (bind _neighbors (Default|ValidateNeighbors (Variables|/Game/_Renato/Revamp_Core/Grid/Blueprints/BP_GenerateGrid.BP_GenerateGrid_C|GetBPGridPathfinding (Variables|/Game/_Renato/Revamp_Core/Player/BP_PlayerActions.BP_PlayerActions_C|GetBP_Grid (Variables|Default|GetPlayerActions))) Index false))
  (for _array_element _neighbors
    (Default|AddStatetoTile (Variables|/Game/_Renato/Revamp_Core/Player/BP_PlayerActions.BP_PlayerActions_C|GetBP_Grid (Variables|Default|GetPlayerActions)) (.Index (Utilities|Struct|BreakS_PathfindingData _array_element)) "NewEnumerator4")))