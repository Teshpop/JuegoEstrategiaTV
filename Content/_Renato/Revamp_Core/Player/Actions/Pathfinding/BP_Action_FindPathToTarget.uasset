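; BP_Action_FindPathToTarget is a player grid action that finds and highlights a path from the selected tile to a target tile.
; ExecuteAction clears one tile state, runs the grid pathfinding component's FindPath with its diagonal setting, then applies that state to every tile on the returned path.
; On destruction, it re-executes with an off-grid sentinel index, which clears the existing highlight.
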(event EventDestroyed
  (CallFunction|ExecuteAction (Utilities|Struct|MakeIntPoint -999 -999)))

(fn ConstructionScript
  (|CallParentFunction))

(fn ExecuteAction
  (params (Index :type Int%20Point%20Structure))
  (bind _playeractions (Variables|Default|GetPlayerActions))
  (bind _bp_grid (Variables|/Game/_Renato/Revamp_Core/Player/BP_PlayerActions.BP_PlayerActions_C|GetBP_Grid _playeractions))
  (bind _bpgridpathfinding (Variables|/Game/_Renato/Revamp_Core/Grid/Blueprints/BP_GenerateGrid.BP_GenerateGrid_C|GetBPGridPathfinding _bp_grid))
  (Default|ClearAllTIleStates (Variables|/Game/_Renato/Revamp_Core/Player/BP_PlayerActions.BP_PlayerActions_C|GetBP_Grid (Variables|Default|GetPlayerActions)) "NewEnumerator4")
  (bind _path (Default|FindPath _bpgridpathfinding (Variables|/Game/_Renato/Revamp_Core/Player/BP_PlayerActions.BP_PlayerActions_C|GetSelectedTile (Variables|Default|GetPlayerActions)) Index (Variables|/Game/_Renato/Revamp_Core/Grid/Blueprints/BP_GridPathfinding.BP_GridPathfinding_C|GetUseTileDiagonals? _bpgridpathfinding)))
  (for _array_element _path
    (Default|AddStatetoTile (Variables|/Game/_Renato/Revamp_Core/Player/BP_PlayerActions.BP_PlayerActions_C|GetBP_Grid (Variables|Default|GetPlayerActions)) _array_element "NewEnumerator4")))