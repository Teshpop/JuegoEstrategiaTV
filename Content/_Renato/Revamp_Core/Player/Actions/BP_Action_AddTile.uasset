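; Player action that adds a new tile to the grid at a given index.
; ExecuteAction acts only when that index is not already valid on the grid owned by PlayerActions.
; It traces the ground at the tile's location, then registers tile data with a fixed tile type, the traced position, zero rotation and the grid's tile scale.
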(fn ConstructionScript
  (|CallParentFunction))

(fn ExecuteAction
  (params (Index :type Int%20Point%20Structure))
  (bind (_x _y) (Utilities|Struct|BreakIntPoint Index))
  (if (not (Default|IsIndexValid (Variables|/Game/_Renato/Revamp_Core/Player/BP_PlayerActions.BP_PlayerActions_C|GetBP_Grid (Variables|Default|GetPlayerActions)) Index))
    (bind _outlocation (Default|TraceGround (Variables|/Game/_Renato/Revamp_Core/Player/BP_PlayerActions.BP_PlayerActions_C|GetBP_Grid (Variables|Default|GetPlayerActions)) (Default|GetTileLocation (Variables|/Game/_Renato/Revamp_Core/Player/BP_PlayerActions.BP_PlayerActions_C|GetBP_Grid (Variables|Default|GetPlayerActions)) _x _y)))
    (Default|AddGridTile (Variables|/Game/_Renato/Revamp_Core/Player/BP_PlayerActions.BP_PlayerActions_C|GetBP_Grid (Variables|Default|GetPlayerActions)) (Utilities|Struct|MakeS_TileData Index "NewEnumerator1" (Math|Transform|MakeTransform _outlocation "0, 0, 0" (Default|GetTileScale (Variables|/Game/_Renato/Revamp_Core/Player/BP_PlayerActions.BP_PlayerActions_C|GetBP_Grid (Variables|Default|GetPlayerActions)))) "NewEnumerator0"))))