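; Player input actor for the tile grid that runs swappable left- and right-click actions on the tile under the cursor.
; Tick tracks the hovered tile through BP_GenerateGrid, updating its tile state and signaling changes.
; Clicks execute the spawned action actors, and hover changes re-execute them while their button flag is set.
; SetSelectedActions spawns these actions, defaulting to add unit (left) and find path (right).
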(event Custom|OnHoveredTileChange
  (Utilities|FlowControl|Sequence
    (:then_0
      (if (Variables|Default|GetIsLeftClickDown?)
        (Variables|Default|GetSelectedAction_LeftClick
          (:then
            (Default|ExecuteAction (Variables|Default|GetSelectedAction_LeftClick) (Variables|Default|GetHoveredTile)))
          (:else))))
    (:then_1
      (if (Variables|Default|GetIsRightClickDown?)
        (Variables|Default|GetSelectedAction_RightClick
          (:then
            (Default|ExecuteAction (Variables|Default|GetSelectedAction_RightClick) (Variables|Default|GetHoveredTile)))
          (:else))))))

(event EventBeginPlay
  (bind _returnvalue (Actor|GetActorOfClass "/Game/_Renato/Revamp_Core/Grid/Blueprints/BP_GenerateGrid.BP_GenerateGrid_C"))
  (Variables|Default|SetBP_Grid _returnvalue)
  (bind _returnvalue_2 (Actor|GetActorOfClass "/Game/_Renato/Revamp_Core/Combat/Blueprints/BP_CombatManager.BP_CombatManager_C"))
  (Variables|Default|SetBPCombatManager _returnvalue_2)
  (Input|EnableInput (Game|GetPlayerController 0))
  (CallFunction|SetSelectedActions "/Game/_Renato/Revamp_Core/Player/Actions/BP_Action_AddUnitToMap.BP_Action_AddUnitToMap_C" "/Game/_Renato/Revamp_Core/Player/Actions/Pathfinding/BP_Action_FindPathToTarget.BP_Action_FindPathToTarget_C"))

(event EventTick
  (params (DeltaSeconds :type Float%20%28single-precision%29))
  (CallFunction|UpdateTileCursor))

(event Input|MouseEvents|LeftMouseButton
  (params (Key :type Key%20Structure :default "None"))
  (:Pressed
    (CallFunction|UpdateTileCursor)
    (Variables|Default|SetIsLeftClickDown? true) ; Execute whilst held
    (Variables|Default|GetSelectedAction_LeftClick
      (:then
        (Default|ExecuteAction (Variables|Default|GetSelectedAction_LeftClick) (Variables|Default|GetHoveredTile)))
      (:else)))
  (:Released
    (Variables|Default|SetIsLeftClickDown? false)))

(event Input|MouseEvents|RightMouseButton
  (params (Key :type Key%20Structure :default "None"))
  (:Pressed
    (CallFunction|UpdateTileCursor)
    (Variables|Default|SetIsRightClickDown? true)
    (Variables|Default|GetSelectedAction_RightClick
      (:then
        (Default|ExecuteAction (Variables|Default|GetSelectedAction_RightClick) (Variables|Default|GetHoveredTile)))
      (:else)))
  (:Released
    (Variables|Default|SetIsLeftClickDown? false)))

(fn ConstructionScript)

(fn UpdateTileCursor
  (bind _index (Default|GetTileIndexUnderCursor (Variables|Default|GetBP_Grid)))
  (if (!= _index (Variables|Default|GetHoveredTile))
    (Default|RemoveStatefromTile (Variables|Default|GetBP_Grid) (Variables|Default|GetHoveredTile) "NewEnumerator1")
    (Variables|Default|SetHoveredTile _index)
    (Default|AddStatetoTile (Variables|Default|GetBP_Grid) (Variables|Default|GetHoveredTile) "NewEnumerator1")
    (CallFunction|OnHoveredTileChange)))

(fn SetSelectedActions
  (params (LeftAction :type BP%20Action%20Class%20Reference) (RightAction :type BP%20Action%20Class%20Reference))
  (Utilities|FlowControl|Sequence
    (:then_0
      (Variables|Default|GetSelectedAction_LeftClick
        (:then
          (Actor|DestroyActor)
          (Variables|Default|SetSelectedAction_LeftClick 0))
        (:else
          _))
      (if (Utilities|IsValidClass LeftAction)
        (bind _returnvalue (Game|SpawnActorfromClass LeftAction (Math|Transform|MakeTransform "0, 0, 0") "AlwaysSpawn" "MultiplyWithRoot" 0 self 0))
        (Variables|Default|SetSelectedAction_LeftClick _returnvalue)))
    (:then_1
      (Variables|Default|GetSelectedAction_RightClick
        (:then
          (Actor|DestroyActor)
          (Variables|Default|SetSelectedAction_RightClick 0))
        (:else
          _))
      (if (Utilities|IsValidClass RightAction)
        (bind _returnvalue_2 (Game|SpawnActorfromClass RightAction (Math|Transform|MakeTransform "0, 0, 0") "AlwaysSpawn" "MultiplyWithRoot" 0 self 0))
        (Variables|Default|SetSelectedAction_RightClick _returnvalue_2)))))