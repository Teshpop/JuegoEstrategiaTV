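; BP_TestTroop is a player camera rig with pan, zoom, orbit and pitch controls that also creates the HUD on BeginPlay.
; Enhanced Input events set clamped targets for actor location, spring arm length, yaw and pitch, with panning derived from the camera's orientation.
; Tick interpolates location, arm length and yaw toward those targets for smooth motion, while pitch from the dolly input applies without smoothing.
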(event Input|EnhancedActionEvents|EnhancedInputActionIA_Dollying
  (params (ActionValue :type Vector%202D%20Structure) (ElapsedSeconds :type Float%20%28double-precision%29) (TriggeredSeconds :type Float%20%28double-precision%29) (InputAction :type Input%20Action%20Object%20Reference :default "/Game/_Renato/Revamp_Core/MappingContext/IA_Dollying.IA_Dollying"))
  ;[0 0.4385 1] Camera Rotation
  (Variables|Default|SetDesiredDolly (Math|Rotator|MakeRotator 0.0 (Math|Float|Clamp(Float) (.Pitch (Math|Rotator|BreakRotator (Math|Rotator|CombineRotators (Variables|Default|GetDesiredDolly) (Math|Rotator|MakeRotator 0.0 (* (* (.Y (Math|Vector2D|BreakVector2D ActionValue)) (Variables|Default|GetOrbitSpeed)) -1.0) 0.0)))) -89.0 -15.0) 0.0)))

(event Input|EnhancedActionEvents|EnhancedInputActionIA_Zoom
  (params (ActionValue :type Float%20%28double-precision%29) (ElapsedSeconds :type Float%20%28double-precision%29) (TriggeredSeconds :type Float%20%28double-precision%29) (InputAction :type Input%20Action%20Object%20Reference :default "/Game/_Renato/Revamp_Core/MappingContext/IA_Zoom.IA_Zoom"))
  ;[0 0.4341 1] Camera Zoom
  (Variables|Default|SetNextPoint (Math|Float|Clamp(Float) (- (Variables|Default|GetNextPoint) (* ActionValue (Variables|Default|GetZoomSpeed))) 1.95e+03 8.95e+03)))

(event Input|EnhancedActionEvents|EnhancedInputActionIA_Panning
  (params (ActionValue :type Vector%202D%20Structure) (ElapsedSeconds :type Float%20%28double-precision%29) (TriggeredSeconds :type Float%20%28double-precision%29) (InputAction :type Input%20Action%20Object%20Reference :default "/Game/_Renato/Revamp_Core/MappingContext/IA_Panning.IA_Panning"))
  (bind (_x _y) (Math|Vector2D|BreakVector2D ActionValue))
  (bind _springarm (Variables|Default|GetSpringArm))
  (bind _returnvalue (Transformation|GetWorldRotation _springarm))
  ;[0 0.4428 1] Pass Input values for interpolation
  (Variables|Default|SetDesiredLocation (Math|Vector|ClampVectorSize (+ (Variables|Default|GetDesiredLocation) (Math|Vector|MakeVector (.Y (Math|Vector|BreakVector (* (* _y (Variables|Default|GetPanningSpeed)) (Math|Vector|GetRightVector _returnvalue)))) (.X (Math|Vector|BreakVector (* (Math|Vector|GetForwardVector _returnvalue) (* _x (Variables|Default|GetPanningSpeed))))) 0.0)) -4.5e+03 4.5e+03)))

(event Input|EnhancedActionEvents|EnhancedInputActionIA_Orbit
  (params (ActionValue :type Vector%202D%20Structure) (ElapsedSeconds :type Float%20%28double-precision%29) (TriggeredSeconds :type Float%20%28double-precision%29) (InputAction :type Input%20Action%20Object%20Reference :default "/Game/_Renato/Revamp_Core/MappingContext/IA_Orbit.IA_Orbit"))
  ;[0 0.4385 1] Camera Rotation
  (Variables|Default|SetDesiredOrbit (Math|Rotator|MakeRotator 0.0 0.0 (Math|Float|Clamp(Float) (.Yaw (Math|Rotator|BreakRotator (Math|Rotator|CombineRotators (Variables|Default|GetDesiredOrbit) (Math|Rotator|MakeRotator 0.0 0.0 (* (.X (Math|Vector2D|BreakVector2D ActionValue)) (Variables|Default|GetOrbitSpeed)))))) -1.8e+02 1.8e+02))))

(event EventTick
  (params (DeltaSeconds :type Float%20%28single-precision%29))
  (bind _springarm (Variables|Default|GetSpringArm))
  (bind _desireddolly (Variables|Default|GetDesiredDolly))
  (bind _pitch (Math|Rotator|BreakRotator _desireddolly))
  ;[0 0.5166 1] Interpolate to smooth transition
  (Variables|/Script/Engine.SpringArmComponent|SetTargetArmLength _springarm (Math|Interpolation|FInterpTo (Variables|/Script/Engine.SpringArmComponent|GetTargetArmLength _springarm) (Variables|Default|GetNextPoint) DeltaSeconds 2.0))
  ;[0 0.5032 1] Camera Panning
  (Transformation|SetActorLocation (Math|Interpolation|VInterpTo (Transformation|GetActorLocation) (Variables|Default|GetDesiredLocation) DeltaSeconds 5.0) false false)
  ;[0 0.3928 1] Interpolate camera rotastion
  (Transformation|SetWorldRotation (Variables|Default|GetSpringArm) (Math|Interpolation|RInterpTo (Math|Rotator|MakeRotator 0.0 _pitch (.Yaw (Math|Rotator|BreakRotator (Transformation|GetWorldRotation (Variables|Default|GetSpringArm))))) (Math|Rotator|MakeRotator 0.0 _pitch (.Yaw (Math|Rotator|BreakRotator (Variables|Default|GetDesiredOrbit)))) DeltaSeconds 5.0) false false))

(event EventBeginPlay
  ;[0 0.5856 1] Initialize objects position
  (Variables|Default|SetDesiredLocation (Transformation|GetActorLocation))
  (Variables|Default|SetNextPoint (Variables|/Script/Engine.SpringArmComponent|GetTargetArmLength (Variables|Default|GetSpringArm)))
  (Variables|Default|SetDesiredOrbit (Math|Rotator|MakeRotator 0.0 0.0 (.Yaw (Math|Rotator|BreakRotator (Transformation|GetWorldRotation (Variables|Default|GetSpringArm))))))
  (Variables|Default|SetDesiredDolly (Math|Rotator|MakeRotator 0.0 (.Pitch (Math|Rotator|BreakRotator (Transformation|GetWorldRotation (Variables|Default|GetSpringArm)))) 0.0))
  (bind _returnvalue (UserInterface|CreateWidget "/Game/_Renato/Revamp_Core/Widgets/WBP_HUD.WBP_HUD_C"))
  (UserInterface|Viewport|AddtoViewport _returnvalue 0))

(fn ConstructionScript)