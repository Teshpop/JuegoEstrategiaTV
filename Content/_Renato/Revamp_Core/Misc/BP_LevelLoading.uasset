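; BP_LevelLoading is a Blueprint that loads a streaming level by name, starting with its LoadedLevel on BeginPlay.
; LoadLevel acts when forced or when the requested name differs from LoadedLevel, then stores that name and sets the level loaded and visible, printing an error if invalid.
; Its preceding unload step targets the requested level instead of the previous LoadedLevel, so previously loaded levels are left untouched.
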(event EventBeginPlay
  (CallFunction|LoadLevel (Variables|Default|GetLoadedLevel) true))

(fn ConstructionScript)

(fn LoadLevel
  (params (LevelToLoad :type String) (ForceLoad :type Boolean))
  (bind _returnvalue (Utilities|String|StringToName LevelToLoad))
  (bind _returnvalue_2 (Utilities|String|StringToName LevelToLoad))
  (bind _returnvalue_3 (Class|GameplayStatics|GetStreamingLevel _returnvalue))
  (bind _returnvalue_4 (Class|GameplayStatics|GetStreamingLevel _returnvalue_2))
  (if (or ForceLoad (Utilities|Enum|NotEqual(Enum) LevelToLoad (Variables|Default|GetLoadedLevel)))
    (Utilities|FlowControl|Sequence
      (:then_0
        (Utilities|IsValid _returnvalue_4
          (:Is%20Valid
            (Variables|/Script/Engine.LevelStreaming|SetbShouldBeLoaded _returnvalue_4 false)
            (Variables|/Script/Engine.LevelStreaming|SetbShouldBeVisible _returnvalue_4 false))))
      (:then_1
        (bind _output_get (Variables|Default|SetLoadedLevel LevelToLoad))
        (Utilities|IsValid _returnvalue_3
          (:Is%20Valid
            (Variables|/Script/Engine.LevelStreaming|SetbShouldBeLoaded _returnvalue_3 true)
            (Variables|/Script/Engine.LevelStreaming|SetbShouldBeVisible _returnvalue_3 true))
          (:Is%20Not%20Valid
            (Development|PrintString (Utilities|String|Append "Error - Load level / Invalid Level name" _output_get) true true "(R=0.000000,G=0.660000,B=1.000000,A=1.000000)" 5.0)))))))