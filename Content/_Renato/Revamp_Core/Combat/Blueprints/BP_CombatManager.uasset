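; BP_CombatManager tracks units in grid-based combat and keeps their placement in sync with BPGrid.
; AddUnitToCombat registers a unit, then SetUnitIndexOnGride releases its previous tile, updates its index and writes it into the new tile's data.
; A sentinel index marks units as off-grid.
; Units snap to their tile's location, or move far away when the index has no tile.
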(event EventBeginPlay)

(event Collision|EventActorBeginOverlap
  (params (OtherActor :type Actor%20Object%20Reference)))

(event EventTick
  (params (DeltaSeconds :type Float%20%28single-precision%29)))

(fn ConstructionScript)

(fn AddUnittoCombat
  (params (BP_Unit :type BP%20Troop%20Debug%20Object%20Reference) (Index :type Int%20Point%20Structure))
  (Utilities|Array|Add (Variables|Default|GetUnitsInCombat) BP_Unit)
  (CallFunction|SetUnitIndexonGride BP_Unit Index))

(fn SetUnitIndexonGride
  (params (BP_Unit :type BP%20Troop%20Debug%20Object%20Reference) (Index :type Int%20Point%20Structure))
  (Utilities|FlowControl|Sequence
    (:then_0
      (if (!= (Variables|/Game/_Renato/ObjectPlacement/BP_TroopDebug.BP_TroopDebug_C|GetIndex BP_Unit) Index)
        (Utilities|FlowControl|Sequence
          (:then_0
            (bind _output_get (LocalVariables|SetPreviousTile (.Value (Utilities|Map|Find (Variables|/Game/_Renato/Revamp_Core/Grid/Blueprints/BP_GenerateGrid.BP_GenerateGrid_C|GetGridTiles (Variables|Default|GetBPGrid)) (Variables|/Game/_Renato/ObjectPlacement/BP_TroopDebug.BP_TroopDebug_C|GetIndex BP_Unit)))))
            (if (== (.UnitOnTile (Utilities|Struct|BreakS_TileData _output_get)) BP_Unit)
              (bind _structout (Utilities|Struct|SetmembersinS_TileData (LocalVariables|GetPreviousTile)))
              (Utilities|Map|Add (Variables|/Game/_Renato/Revamp_Core/Grid/Blueprints/BP_GenerateGrid.BP_GenerateGrid_C|GetGridTiles (Variables|Default|GetBPGrid)) (.Index (Utilities|Struct|BreakS_TileData _structout)) _structout)))
          (:then_1
            (Variables|/Game/_Renato/ObjectPlacement/BP_TroopDebug.BP_TroopDebug_C|SetIndex BP_Unit Index)
            (if (!= Index (Utilities|Struct|MakeIntPoint -999 -999))
              (bind _structout_2 (Utilities|Struct|SetmembersinS_TileData (.Value (Utilities|Map|Find (Variables|/Game/_Renato/Revamp_Core/Grid/Blueprints/BP_GenerateGrid.BP_GenerateGrid_C|GetGridTiles (Variables|Default|GetBPGrid)) Index)) BP_Unit))
              (Utilities|Map|Add (Variables|/Game/_Renato/Revamp_Core/Grid/Blueprints/BP_GenerateGrid.BP_GenerateGrid_C|GetGridTiles (Variables|Default|GetBPGrid)) (.Index (Utilities|Struct|BreakS_TileData _structout_2)) _structout_2))))))
    (:then_1
      (Transformation|SetActorLocation BP_Unit (select (.ReturnValue (Utilities|Map|Find (Variables|/Game/_Renato/Revamp_Core/Grid/Blueprints/BP_GenerateGrid.BP_GenerateGrid_C|GetGridTiles (Variables|Default|GetBPGrid)) Index)) (.Location (Math|Transform|BreakTransform (.Transform (Utilities|Struct|BreakS_TileData (.Value (Utilities|Map|Find (Variables|/Game/_Renato/Revamp_Core/Grid/Blueprints/BP_GenerateGrid.BP_GenerateGrid_C|GetGridTiles (Variables|Default|GetBPGrid)) Index)))))) "-999999.000000,-999999.000000,-999999.000000") false false))))