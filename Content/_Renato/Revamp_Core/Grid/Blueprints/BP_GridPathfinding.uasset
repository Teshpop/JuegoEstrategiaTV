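; Grid pathfinder that uses A* to return a tile path from a start to a target index, excluding the start.
; Neighbors come from square grids, with optional diagonals, filtered by walkability and climbable height difference.
; Discovered tiles sit in parallel arrays sorted by cost plus a Chebyshev or Manhattan heuristic.
; The search stops when the target is first discovered, then rebuilds the path through previous-tile links.
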(event EventBeginPlay)

(fn ConstructionScript)

(fn GetTileNeighbors
  (params (Index :type Int%20Point%20Structure) (UseDiagonals :type Boolean))
  (switch Utilities|FlowControl|Switch|SwitchonE_GridTypes (Variables|/Game/_Renato/Revamp_Core/Grid/Blueprints/BP_GenerateGrid.BP_GenerateGrid_C|GetGridType (Variables|Default|GetGrid))
    (:NewEnumerator1
      (return (CallFunction|GetSquareNeighborIndexes Index (Variables|Default|GetUseTileDiagonals?))))))

(fn GetSquareNeighborIndexes
  (params (Index :type Int%20Point%20Structure) (UseDiagonals :type Boolean))
  (bind _intpoint (Utilities|Struct|MakeIntPoint 1 0))
  (bind _intpoint_2 (Utilities|Struct|MakeIntPoint 0 1))
  (bind _intpoint_3 (Utilities|Struct|MakeIntPoint -1 0))
  (bind _intpoint_4 (Utilities|Struct|MakeIntPoint 0 -1))
  (bind _returnvalue (+ Index _intpoint))
  (bind _returnvalue_2 (+ Index _intpoint_2))
  (bind _returnvalue_3 (+ Index _intpoint_3))
  (bind _returnvalue_4 (+ Index _intpoint_4))
  (bind _array (Utilities|Array|MakeArray _returnvalue _returnvalue_2 _returnvalue_3 _returnvalue_4))
  (if UseDiagonals
    (LocalVariables|SetReturnValue _array)
    (Utilities|Array|AppendArray (LocalVariables|GetReturnValue) (Utilities|Array|MakeArray (+ Index (Utilities|Struct|MakeIntPoint 1 1)) (+ Index (Utilities|Struct|MakeIntPoint -1 1)) (+ Index (Utilities|Struct|MakeIntPoint -1 -1)) (+ Index (Utilities|Struct|MakeIntPoint 1 -1))))
    (return (LocalVariables|GetReturnValue))
    (else
      (return _array))))

(fn ValidateNeighbors
  (params (Index :type Int%20Point%20Structure) (UseDiagonals :type Boolean))
  (LocalVariables|SetInputData (.Value (Utilities|Map|Find (Variables|/Game/_Renato/Revamp_Core/Grid/Blueprints/BP_GenerateGrid.BP_GenerateGrid_C|GetGridTiles (Variables|Default|GetGrid)) Index)))
  (bind _neighbors (CallFunction|GetTileNeighbors Index UseDiagonals))
  (for _array_element _neighbors
    (LocalVariables|SetData (.Value (Utilities|Map|Find (Variables|/Game/_Renato/Revamp_Core/Grid/Blueprints/BP_GenerateGrid.BP_GenerateGrid_C|GetGridTiles (Variables|Default|GetGrid)) _array_element)))
    (if (CallFunction|IsTileWalkable (.TileType (Utilities|Struct|BreakS_TileData (LocalVariables|GetData))))
      (if (<= (Math|Float|Absolute(Float) (- (.Z (Math|Vector|BreakVector (.Location (Math|Transform|BreakTransform (.Transform (Utilities|Struct|BreakS_TileData (LocalVariables|GetData))))))) (.Z (Math|Vector|BreakVector (.Location (Math|Transform|BreakTransform (.Transform (Utilities|Struct|BreakS_TileData (LocalVariables|GetInputData))))))))) (* (.Z (Math|Vector|BreakVector (Variables|/Game/_Renato/Revamp_Core/Grid/Blueprints/BP_GenerateGrid.BP_GenerateGrid_C|GetGridTileSize (Variables|Default|GetGrid)))) (Variables|Default|GetHeightClimbDistance)))
        (Utilities|Array|Add (LocalVariables|GetReturnNeighbors) (Utilities|Struct|MakeS_PathfindingData (.Index (Utilities|Struct|BreakS_TileData (LocalVariables|GetData))) 1 999999 999999 Index)))))
  (return (LocalVariables|GetReturnNeighbors)))

(fn FindPath
  (params (Start :type Int%20Point%20Structure) (Target :type Int%20Point%20Structure) (Diagonals :type Boolean))
  (Variables|Default|SetStartTileIndex Start)
  (Variables|Default|SetTargetTileIndex Target)
  (Variables|Default|SetUseTileDiagonals? Diagonals)
  (CallFunction|CleanGeneratedData)
  (bind _isvalid (CallFunction|ValidateInputData))
  (if _isvalid
    (CallFunction|DiscoverTile (Utilities|Struct|MakeS_PathfindingData (Variables|Default|GetStartTileIndex) 1 0 (CallFunction|GetMinimumCostBetween2Tiles (Variables|Default|GetStartTileIndex) (Variables|Default|GetTargetTileIndex) (Variables|Default|GetUseTileDiagonals?))))
    (while (> (Utilities|Array|Length (Variables|Default|GetDiscoveredTilesIndexes)) 0)
      (bind _foundtargettile (CallFunction|AnalyzeNextDiscoveredTile))
      (if _foundtargettile
        (bind _path (CallFunction|GeneratePath))
        (return _path)))
    (return (Utilities|Array|MakeArray))
    (else
      (return (Utilities|Array|MakeArray)))))

(fn ValidateInputData
  (if (!= (Variables|Default|GetStartTileIndex) (Variables|Default|GetTargetTileIndex))
    (if (Default|IsTileWalkable (Variables|Default|GetGrid) (Variables|Default|GetStartTileIndex))
      (if (Default|IsTileWalkable (Variables|Default|GetGrid) (Variables|Default|GetTargetTileIndex))
        (return true)
        (else
          (return false)))
      (else
        (return false)))
    (else
      (return false))))

(fn DiscoverTile
  (params (TilePathData :type S%20Pathfinding%20Data%20Structure))
  (Utilities|Map|Add (Variables|Default|GetPathfindingData) (.Index (Utilities|Struct|BreakS_PathfindingData TilePathData)) TilePathData)
  (CallFunction|InsertTileinDiscoveredArray TilePathData))

(fn GetMinimumCostBetween2Tiles
  (params (StartIndex :type Int%20Point%20Structure) (DestinationIndex :type Int%20Point%20Structure) (Diagonals :type Boolean))
  (bind _returnvalue (- StartIndex DestinationIndex))
  (bind _returnvalue_2 (- StartIndex DestinationIndex))
  (bind (_x _y) (Utilities|Struct|BreakIntPoint _returnvalue))
  (bind (_x_2 _y_2) (Utilities|Struct|BreakIntPoint _returnvalue_2))
  (if (Variables|Default|GetUseTileDiagonals?)
    (return (Math|Integer|Max(Integer) (Math|Integer|Absolute(Integer) _x_2) (Math|Integer|Absolute(Integer) _y_2)))
    (else
      (return (+ (Math|Integer|Absolute(Integer) _x) (Math|Integer|Absolute(Integer) _y))))))

(fn AnalyzeNextDiscoveredTile
  (bind _tilepathdata (CallFunction|SelectCheapestTile))
  (Variables|Default|SetCurrentlyDiscoveredTile _tilepathdata)
  (bind _neighbors (CallFunction|ValidateNeighbors (.Index (Utilities|Struct|BreakS_PathfindingData (Variables|Default|GetCurrentlyDiscoveredTile))) (Variables|Default|GetUseTileDiagonals?)))
  (Variables|Default|SetCurrentNeighbors _neighbors)
  (while (> (Utilities|Array|Length (Variables|Default|GetCurrentNeighbors)) 0)
    (bind _istargettile_ (CallFunction|DiscoverNextNeighbor))
    (if _istargettile_
      (return true)))
  (return false))

(fn GeneratePath
  (LocalVariables|SetCurrent (Variables|Default|GetTargetTileIndex))
  (while (!= (LocalVariables|GetCurrent) (Variables|Default|GetStartTileIndex))
    (Utilities|Array|Add (LocalVariables|GetInvertedPath) (LocalVariables|GetCurrent))
    (LocalVariables|SetCurrent (.PreviousIndex (Utilities|Struct|BreakS_PathfindingData (.Value (Utilities|Map|Find (Variables|Default|GetPathfindingData) (LocalVariables|GetCurrent)))))))
  (bind _arrayelement (Utilities|Array|ReverseforEachLoop (LocalVariables|GetInvertedPath))
    (:LoopBody
      (Utilities|Array|Add (LocalVariables|GetReturnedPath) _arrayelement))
    (:Completed
      (return (LocalVariables|GetReturnedPath)))))

(fn SelectCheapestTile
  (LocalVariables|SetTileIndex (Utilities|Array|Get(acopy) (Variables|Default|GetDiscoveredTilesIndexes)))
  (Utilities|Array|RemoveIndex (Variables|Default|GetDiscoveredTilesSortingCost))
  (Utilities|Array|RemoveIndex (Variables|Default|GetDiscoveredTilesIndexes))
  (Utilities|Array|Add (Variables|Default|GetAnalyzedTileIndexes) (LocalVariables|GetTileIndex))
  (return (.Value (Utilities|Map|Find (Variables|Default|GetPathfindingData) (LocalVariables|GetTileIndex)))))

(fn DiscoverNextNeighbor
  (bind _targettileindex (Variables|Default|GetTargetTileIndex))
  (bind (_x _y) (Utilities|Struct|BreakIntPoint _targettileindex))
  (Variables|Default|SetCurrentNeighbor (Utilities|Array|Get(acopy) (Variables|Default|GetCurrentNeighbors)))
  (Utilities|Array|RemoveIndex (Variables|Default|GetCurrentNeighbors))
  (if (not (Utilities|Array|ContainsItem (Variables|Default|GetAnalyzedTileIndexes) (.Index (Utilities|Struct|BreakS_PathfindingData (Variables|Default|GetCurrentNeighbor)))))
    (LocalVariables|SetCostFromStart (+ (.CostFromStart (Utilities|Struct|BreakS_PathfindingData (Variables|Default|GetCurrentlyDiscoveredTile))) (.CostToEnterTile (Utilities|Struct|BreakS_PathfindingData (Variables|Default|GetCurrentNeighbor)))))
    (bind _output_get (LocalVariables|SetIndexDiscovered (Utilities|Array|FindItem (Variables|Default|GetDiscoveredTilesIndexes) (.Index (Utilities|Struct|BreakS_PathfindingData (Variables|Default|GetCurrentNeighbor))))))
    (if (== _output_get -1)
      _
      (else
        (bind _output_get_2 (Variables|Default|SetCurrentNeighbor (.Value (Utilities|Map|Find (Variables|Default|GetPathfindingData) (.Index (Utilities|Struct|BreakS_PathfindingData (Variables|Default|GetCurrentNeighbor)))))))
        (if (< (LocalVariables|GetCostFromStart) (.CostFromStart (Utilities|Struct|BreakS_PathfindingData _output_get_2)))
          (Utilities|Array|RemoveIndex (Variables|Default|GetDiscoveredTilesIndexes) (LocalVariables|GetIndexDiscovered))
          (Utilities|Array|RemoveIndex (Variables|Default|GetDiscoveredTilesSortingCost) (LocalVariables|GetIndexDiscovered))
          (else
            (return false)))))
    (CallFunction|DiscoverTile (Utilities|Struct|MakeS_PathfindingData (.Index (Utilities|Struct|BreakS_PathfindingData (Variables|Default|GetCurrentNeighbor))) (.CostToEnterTile (Utilities|Struct|BreakS_PathfindingData (Variables|Default|GetCurrentNeighbor))) (LocalVariables|GetCostFromStart) (CallFunction|GetMinimumCostBetween2Tiles (.Index (Utilities|Struct|BreakS_PathfindingData (Variables|Default|GetCurrentNeighbor))) (Variables|Default|GetTargetTileIndex) (Variables|Default|GetUseTileDiagonals?)) (.Index (Utilities|Struct|BreakS_PathfindingData (Variables|Default|GetCurrentlyDiscoveredTile)))))
    (if (and (== (.X (Utilities|Struct|BreakIntPoint (.Index (Utilities|Struct|BreakS_PathfindingData (Variables|Default|GetCurrentNeighbor))))) _x) (== _y (.Y (Utilities|Struct|BreakIntPoint (.Index (Utilities|Struct|BreakS_PathfindingData (Variables|Default|GetCurrentNeighbor)))))))
      (return true)
      (else
        (return false)))
    (else
      (return false))))

(fn InsertTileinDiscoveredArray
  (params (TileData :type S%20Pathfinding%20Data%20Structure))
  (bind (_index _costtoentertile _costfromstart _minimumcosttotarget) (Utilities|Struct|BreakS_PathfindingData TileData))
  (bind _discoveredtilessortingcost (Variables|Default|GetDiscoveredTilesSortingCost))
  (LocalVariables|SetSortingCost (+ _costfromstart _minimumcosttotarget))
  (if (== (Utilities|Array|Length (Variables|Default|GetDiscoveredTilesSortingCost)) 0)
    (Utilities|Array|Add (Variables|Default|GetDiscoveredTilesSortingCost) (LocalVariables|GetSortingCost) :!label _label)
    (Utilities|Array|Add (Variables|Default|GetDiscoveredTilesIndexes) (.Index (Utilities|Struct|BreakS_PathfindingData TileData)))
    (elif (>= (LocalVariables|GetSortingCost) (Utilities|Array|Get(acopy) _discoveredtilessortingcost (Utilities|Array|LastIndex _discoveredtilessortingcost)))
      (goto _label)
      (else
        (bind (_array_element _array_index) (Utilities|Array|ForEachLoopwithBreak (Variables|Default|GetDiscoveredTilesSortingCost) :!label _label_2)
          (:LoopBody
            (if (>= _array_element (LocalVariables|GetSortingCost))
              (Utilities|Array|Insert (Variables|Default|GetDiscoveredTilesSortingCost) (LocalVariables|GetSortingCost) _array_index)
              (Utilities|Array|Insert (Variables|Default|GetDiscoveredTilesIndexes) (.Index (Utilities|Struct|BreakS_PathfindingData TileData)) _array_index)
              (goto _label_2 Break))))))))

(fn CleanGeneratedData
  (Utilities|Map|Clear (Variables|Default|GetPathfindingData))
  (Utilities|Array|Clear (Variables|Default|GetDiscoveredTilesSortingCost))
  (Utilities|Array|Clear (Variables|Default|GetDiscoveredTilesIndexes))
  (Utilities|Array|Clear (Variables|Default|GetAnalyzedTileIndexes)))