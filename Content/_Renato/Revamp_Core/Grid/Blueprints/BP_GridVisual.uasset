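; BP_GridVisual renders the tile grid through a child-actor BP_GridMeshInst that manages mesh instances.
; InitializeGridVisual feeds that actor the current shape's flat mesh and material with query-only collision, then places itself at the origin raised by a ground offset.
; UpdateTileVisual removes a tile's instance and re-adds it with transform and state only if the tile is walkable; DestroyGridVisual clears all instances, and tick is disabled.
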(event EventBeginPlay
  (Actor|Tick|SetActorTickEnabled false))

(event Collision|EventActorBeginOverlap
  (params (OtherActor :type Actor%20Object%20Reference)))

(event EventTick
  (params (DeltaSeconds :type Float%20%28single-precision%29)))

(fn ConstructionScript)

(fn InitializeGridVisual
  (params (Grid :type BP%20Generate%20Grid%20Object%20Reference) (Offset :type Float%20%28double-precision%29))
  (Variables|Default|SetGrid Grid)
  (Variables|Default|SetGridMeshInst (.AsBP%20Grid%20Mesh%20Inst (Utilities|Casting|CastToBP_GridMeshInst (Variables|/Script/Engine.ChildActorComponent|GetChildActor (Variables|Default|GetChildActor_GridMeshInst)))))
  (Default|InitializeGridMeshInst :self (Variables|Default|GetGridMeshInst) :Mesh (.FlatMesh (Utilities|Struct|BreakS_GridShapeData (Default|GetCurrentShapeData (Variables|Default|GetGrid)))) :Material (.FlatMaterial (Utilities|Struct|BreakS_GridShapeData (Default|GetCurrentShapeData (Variables|Default|GetGrid)))) :Collision "QueryOnly")
  (Transformation|SetActorLocation "0, 0, 0" false false)
  (CallFunction|SetOffsetfromGround Offset))

(fn SetOffsetfromGround
  (params (Offset :type Float%20%28double-precision%29))
  (bind _returnvalue (Transformation|GetActorLocation))
  (bind (_x _y) (Math|Vector|BreakVector _returnvalue))
  (Variables|Default|SetOffsetFromGround Offset)
  (Transformation|SetActorLocation (Math|Vector|MakeVector _x _y (Variables|Default|GetOffsetFromGround)) false false))

(fn DestroyGridVisual
  (Default|ClearInstance (Variables|Default|GetGridMeshInst)))

(fn UpdateTileVisual
  (params (TileData :type S%20Tile%20Data%20Structure))
  (bind (_index _tiletype _transform _tilestate) (Utilities|Struct|BreakS_TileData TileData))
  (bind (_index_2 _tiletype_2) (Utilities|Struct|BreakS_TileData TileData))
  (Default|RemoveInstance (Variables|Default|GetGridMeshInst) _index_2)
  (if (CallFunction|IsTileWalkable _tiletype_2)
    (Default|AddInstance (Variables|Default|GetGridMeshInst) _transform _index _tilestate)))