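; Grid actor that builds a tile grid around its location in the construction script and again on BeginPlay.
; Optional sphere traces snap tile height to the ground and take tile types from BP_GridModifier2 actors.
; Tiles live in an index-keyed map; changes update the child BP_GridVisual and fire notifications, and child BP_GridPathfinding receives a grid reference.
; Helpers handle tile states, walkability and cursor-to-index lookup (square only), with plane-intersection fallback.
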(event EventBeginPlay
  (CreateGrid|SpawnGrid (Transformation|GetActorLocation) (Variables|GridInit|GetGridTileSize) (Variables|GridInit|GetGridTileCount) (Variables|GridInit|GetGridType)))

(fn ConstructionScript
  (Variables|GridInit|SetGridVisual (.AsBP%20Grid%20Visual (Utilities|Casting|CastToBP_GridVisual (Variables|/Script/Engine.ChildActorComponent|GetChildActor (Variables|Default|GetChildActor_GridVisual)))))
  (bind _output_get (Variables|Default|SetBPGridPathfinding (.AsBP%20Grid%20Pathfinding (Utilities|Casting|CastToBP_GridPathfinding (Variables|/Script/Engine.ChildActorComponent|GetChildActor (Variables|Default|GetChildActor_GridPathfinding))))))
  (Variables|/Game/_Renato/Revamp_Core/Grid/Blueprints/BP_GridPathfinding.BP_GridPathfinding_C|SetGrid _output_get self)
  ;[1 1 1] debug only
  (CreateGrid|SpawnGrid (Transformation|GetActorLocation) (Variables|GridInit|GetGridTileSize) (Variables|GridInit|GetGridTileCount) (Variables|GridInit|GetGridType)))

(fn SpawnGrid
  (params (CenterLocation :type Vector) (TileSize :type Vector) (TileCount :type Vector%202D%20Structure) (GridType :type E_GridTypes%20Enum :default "NewEnumerator0"))
  (Variables|GridInit|SetGridCenterLocation CenterLocation)
  (Variables|GridInit|SetGridTileSize TileSize)
  (Variables|GridInit|SetGridType GridType)
  (Variables|GridInit|SetGridTileCount (Math|Vector2D|MakeVector2D (Math|Conversions|ToFloat(Integer) (Math|Float|Round (.X (Math|Vector2D|BreakVector2D (Variables|GridInit|GetGridTileCount))))) (Math|Conversions|ToFloat(Integer) (Math|Float|Round (.Y (Math|Vector2D|BreakVector2D (Variables|GridInit|GetGridTileCount)))))))
  (CreateGrid|DestroyGrid)
  (Default|InitializeGridVisual (Variables|GridInit|GetGridVisual) self (Variables|GridInit|GetHeightOffset))
  (bind (_bottomleftcorner _centercorner) (CreateGrid|CalculateCenterandBottomLeft))
  (Variables|GridInit|SetGridCenterLocation _centercorner)
  (Variables|GridInit|SetGridBottomLeftCornerLocation _bottomleftcorner)
  (for _index (range 0 (- (Math|Float|Round (.X (Math|Vector2D|BreakVector2D (Variables|GridInit|GetGridTileCount)))) 1))
    (LocalVariables|SetX _index)
    (for _index_2 (range 0 (- (Math|Float|Round (.Y (Math|Vector2D|BreakVector2D (Variables|GridInit|GetGridTileCount)))) 1))
      (LocalVariables|SetY _index_2)
      (bind _output_get (LocalVariables|SetTileTransform (Math|Transform|MakeTransform (TileStates|GetTileLocation (LocalVariables|GetX) (LocalVariables|GetY)) "0, 0, 0" (TileStates|GetTileScale))))
      (if (Variables|GroundScan|GetEnableEnviromentScan)
        (bind (_outlocation _tiletype) (CreateGrid|TraceGround (.Location (Math|Transform|BreakTransform _output_get))))
        (CreateGrid|AddGridTile (Utilities|Struct|MakeS_TileData (Utilities|Struct|MakeIntPoint (LocalVariables|GetX) (LocalVariables|GetY)) _tiletype (Math|Transform|MakeTransform _outlocation "0, 0, 0" (.Scale (Math|Transform|BreakTransform _output_get))) "NewEnumerator0"))
        (Default|CallOnTileDataUpdated (Utilities|Struct|MakeIntPoint (LocalVariables|GetX) (LocalVariables|GetY)))
        (else
          (CreateGrid|AddGridTile (Utilities|Struct|MakeS_TileData (Utilities|Struct|MakeIntPoint (LocalVariables|GetX) (LocalVariables|GetY)) "NewEnumerator1" (LocalVariables|GetTileTransform) "NewEnumerator0")))))))

(fn GetCurrentShapeData
  (return (CallFunction|GetShapeData (Variables|GridInit|GetGridType))))

(fn DestroyGrid
  (Utilities|Map|Clear (Variables|GridInit|GetGridTiles))
  (Default|DestroyGridVisual (Variables|GridInit|GetGridVisual))
  (Default|CallOnGridDestroyed))

(fn CalculateCenterandBottomLeft
  (bind _gridtilecount (Variables|GridInit|GetGridTileCount))
  (bind (_x _y) (Math|Vector2D|BreakVector2D _gridtilecount))
  (LocalVariables|SetGridCenter (CallFunction|SnapVectortoVector (Variables|GridInit|GetGridCenterLocation) (Variables|GridInit|GetGridTileSize)))
  (return (- (LocalVariables|GetGridCenter) (* (* (- (Variables|GridInit|GetGridTileCount) (Math|Vector2D|MakeVector2D (Math|Float|SelectFloat 0.0 1.0 (CallFunction|IsFloatEven _x)) (Math|Float|SelectFloat 0.0 1.0 (CallFunction|IsFloatEven _y)))) 0.5) (Math|Conversions|ToVector2D(Vector) (Variables|GridInit|GetGridTileSize)))) (LocalVariables|GetGridCenter)))

(fn TraceGround
  (params (TileLocation :type Vector))
  (bind (_x _y) (Math|Vector|BreakVector TileLocation))
  (LocalVariables|SetTraceRadius (Math|Conversions|ToFloat(Integer) (Math|Float|Round (* (.X (Math|Vector|BreakVector (Variables|GridInit|GetGridTileSize))) 0.33))))
  (bind _outhits (Collision|MultiSphereTraceByChannel (+ TileLocation (Variables|GroundScan|GetTraceGridSuperiorLimit)) (- TileLocation (Variables|GroundScan|GetTraceGridInferiorLimit)) 0.0 "TraceTypeQuery3" false 0 "None"))
  (if (> (Utilities|Array|Length _outhits) 0)
    (LocalVariables|SetHitTileType "NewEnumerator1")
    (for _array_element _outhits
      (bind _asbp_grid_modifier_2 (Utilities|Casting|CastToBP_GridModifier2 (.HitActor (Collision|BreakHitResult _array_element)))
        (:then
          (LocalVariables|SetHitTileType (Variables|/Game/_Renato/Revamp_Core/Grid/Blueprints/BP_GridModifier2.BP_GridModifier2_C|GetTileType _asbp_grid_modifier_2)))
        (:CastFailed
          (LocalVariables|SetHeightValue (Math|Float|SnapToGrid(Float) (- (.Z (Math|Vector|BreakVector (.Location (Collision|BreakHitResult _array_element)))) (LocalVariables|GetTraceRadius)) (.Z (Math|Vector|BreakVector (Variables|GridInit|GetGridTileSize))))))))
    (return (Math|Vector|MakeVector _x _y (LocalVariables|GetHeightValue)) (LocalVariables|GetHitTileType))
    (else
      (return TileLocation "NewEnumerator0"))))

(fn IsTileTypeWalkable
  (params (NewParam :type E_TileType%20Enum :default "NewEnumerator0"))
  (return (not (Utilities|Array|ContainsItem (Utilities|Array|MakeArray "NewEnumerator0" "NewEnumerator2") NewParam))))

(fn GetCursorLocationonGrid
  (params (PlayerIndex :type Integer))
  (bind _returnvalue (Game|GetPlayerController PlayerIndex))
  (bind (_hitresult _returnvalue_2) (Game|Player|GetHitResultUnderCursorbyChannel _returnvalue "TraceTypeQuery3" false))
  (bind (_worldlocation _worlddirection) (Game|Player|ConvertMouseLocationToWorldSpace _returnvalue))
  (bind (_hitresult_2 _returnvalue_3) (Game|Player|GetHitResultUnderCursorbyChannel _returnvalue "TraceTypeQuery4" false))
  (if _returnvalue_3
    (return (.Location (Collision|BreakHitResult _hitresult_2)))
    (elif _returnvalue_2
      (return (.Location (Collision|BreakHitResult _hitresult)))
      (elif true
        (return (.Intersection (Class|KismetMathLibrary|LinePlaneIntersection _worldlocation (* _worlddirection 999999.0) (Class|KismetMathLibrary|MakePlanefromPointandNormal (Variables|GridInit|GetGridCenterLocation) "0.000000,0.000000,1.000000"))))
        (else
          (return "-999.000000,-999.000000,-999.000000"))))))

(fn GetTileIndexfromWorldLocation
  (params (Location :type Vector))
  (LocalVariables|SetLocationOnGrid (- Location (Variables|GridInit|GetGridBottomLeftCornerLocation)))
  (switch Utilities|FlowControl|Switch|SwitchonE_GridTypes (Variables|GridInit|GetGridType)
    (:NewEnumerator0
      (return (Utilities|Struct|MakeIntPoint -999 -999)))
    (:NewEnumerator1
      (LocalVariables|SetSnappedLocationOnGrid (Math|Conversions|ToVector2D(Vector) (CallFunction|SnapVectortoVector (LocalVariables|GetLocationOnGrid) (Variables|GridInit|GetGridTileSize))))
      (return (Class|KismetMathLibrary|ToIntPoint(Vector2D) (/ (LocalVariables|GetSnappedLocationOnGrid) (Math|Conversions|ToVector2D(Vector) (Variables|GridInit|GetGridTileSize))))))))

(fn GetTileIndexUnderCursor
  (params (PlayerIndex :type Integer))
  (bind _location (CreateGrid|GetCursorLocationonGrid PlayerIndex))
  (bind _index (CreateGrid|GetTileIndexfromWorldLocation _location))
  (return _index _location))

(fn AddGridTile
  (params (Data :type S%20Tile%20Data%20Structure))
  (Utilities|Map|Add (Variables|GridInit|GetGridTiles) (.Index (Utilities|Struct|BreakS_TileData Data)) Data)
  (Default|UpdateTileVisual (Variables|GridInit|GetGridVisual) Data)
  (Default|CallOnTileDataUpdated (.Index (Utilities|Struct|BreakS_TileData Data))))

(fn AddStatetoTile
  (params (Index :type Int%20Point%20Structure) (TileState :type E_TileState%20Enum :default "NewEnumerator0"))
  (bind _gridtiles (Variables|GridInit|GetGridTiles))
  (bind (_value _returnvalue) (Utilities|Map|Find _gridtiles Index))
  (if _returnvalue
    (bind _output_get (LocalVariables|SetData _value))
    (bind _returnvalue_2 (Utilities|Array|AddUnique (.TileState (Utilities|Struct|BreakS_TileData _output_get)) TileState))
    (if (>= _returnvalue_2 0)
      (Utilities|Map|Add (Variables|GridInit|GetGridTiles) (.Index (Utilities|Struct|BreakS_TileData (LocalVariables|GetData))) (LocalVariables|GetData))
      (Default|UpdateTileVisual (Variables|GridInit|GetGridVisual) (LocalVariables|GetData))
      (Default|CallOnTileDataUpdated Index))))

(fn RemoveStatefromTile
  (params (Index :type Int%20Point%20Structure) (TileState :type E_TileState%20Enum :default "NewEnumerator0"))
  (bind _gridtiles (Variables|GridInit|GetGridTiles))
  (bind (_value _returnvalue) (Utilities|Map|Find _gridtiles Index))
  (if _returnvalue
    (bind _output_get (LocalVariables|SetData _value))
    (bind _returnvalue_2 (Utilities|Array|RemoveItem (.TileState (Utilities|Struct|BreakS_TileData _output_get)) TileState))
    (if _returnvalue_2
      (Utilities|Map|Add (Variables|GridInit|GetGridTiles) (.Index (Utilities|Struct|BreakS_TileData (LocalVariables|GetData))) (LocalVariables|GetData))
      (Default|UpdateTileVisual (Variables|GridInit|GetGridVisual) (LocalVariables|GetData))
      (Default|CallOnTileDataUpdated Index))))

(fn IsIndexValid
  (params (Index :type Int%20Point%20Structure))
  (return (Utilities|Map|Contains (Variables|GridInit|GetGridTiles) Index)))

(fn GetTileScale
  (return (/ (Variables|GridInit|GetGridTileSize) (.MeshSize (Utilities|Struct|BreakS_GridShapeData (CreateGrid|GetCurrentShapeData))))))

(fn GetTileLocation
  (params (InInt :type Integer) (InInt2 :type Integer))
  (return (+ (Variables|GridInit|GetGridBottomLeftCornerLocation) (* (Variables|GridInit|GetGridTileSize) (Math|Vector|MakeVector (Math|Conversions|ToFloat(Integer) InInt) (Math|Conversions|ToFloat(Integer) InInt2) 0.0)))))

(fn RemoveGridTile
  (params (Index :type Int%20Point%20Structure))
  (bind _returnvalue (Utilities|Map|Remove (Variables|GridInit|GetGridTiles) Index))
  (if _returnvalue
    (Default|UpdateTileVisual (Variables|GridInit|GetGridVisual) (Utilities|Struct|MakeS_TileData Index "NewEnumerator0" "0.000000,0.000000,0.000000|0.000000,0.000000,0.000000|1.000000,1.000000,1.000000" "NewEnumerator0"))
    (Default|CallOnTileDataUpdated Index)))

(fn GetAllTileswithState
  (params (State :type E_TileState%20Enum :default "NewEnumerator0"))
  (bind _values (Utilities|Map|Values (Variables|GridInit|GetGridTiles)))
  (for _array_element _values
    (if (Utilities|Array|ContainsItem (.TileState (Utilities|Struct|BreakS_TileData _array_element)) State)
      (Utilities|Array|Add (LocalVariables|GetReturnValue) (.Index (Utilities|Struct|BreakS_TileData _array_element)))))
  (return (LocalVariables|GetReturnValue)))

(fn ClearAllTIleStates
  (params (State :type E_TileState%20Enum :default "NewEnumerator0"))
  (bind _indexes (CallFunction|GetAllTileswithState State))
  (for _array_element _indexes
    (TileStates|RemoveStatefromTile _array_element State)))

(fn IsTileWalkable
  (params (Index :type Int%20Point%20Structure))
  (return (CreateGrid|IsTileTypeWalkable (.TileType (Utilities|Struct|BreakS_TileData (.Value (Utilities|Map|Find (Variables|GridInit|GetGridTiles) Index)))))))