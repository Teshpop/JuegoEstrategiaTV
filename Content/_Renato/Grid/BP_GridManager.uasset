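; BP_GridManager builds a square grid of BP_GridCell actors and provides snapping to the nearest cell position.
; On BeginPlay, PopulateGrid spawns cells in nested X/Y loops using the grid size and cell spacing, centered on the world origin rather than the manager's location, and stores them in GridArray.
; GetClosestGridPosition linearly searches that array and returns the location of the cell nearest a given point.
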(event EventBeginPlay
  (CallFunction|PopulateGrid))

(fn ConstructionScript)

(fn PopulateGrid
  (bind _worldgridsize (Variables|Default|GetWorldGridSize))
  (Utilities|Array|Clear (Variables|Default|GetGridArray))
  (LocalVariables|SetWorldOffset (- (* (* (Variables|Default|GetGridSize) _worldgridsize) 0.5) (* _worldgridsize 0.5)))
  ;[0 0.5232 1] Y loop
  (for _index (range 0 (- (Variables|Default|GetGridSize) 1))
    ;[0 0.4866 1] X loop
    (for _index_2 (range 0 (- (Variables|Default|GetGridSize) 1))
      (bind _returnvalue (Game|SpawnActorfromClass "/Game/_Renato/Grid/BP_GridCell.BP_GridCell_C" (Math|Transform|MakeTransform (Math|Vector|MakeVector (Math|Conversions|ToFloat(Integer) (- (* _index_2 (Variables|Default|GetWorldGridSize)) (Math|Float|Truncate (LocalVariables|GetWorldOffset)))) (Math|Conversions|ToFloat(Integer) (- (* _index (Variables|Default|GetWorldGridSize)) (Math|Float|Truncate (LocalVariables|GetWorldOffset)))) 0.0)) "AlwaysSpawn" "MultiplyWithRoot" 0 0))
      (Utilities|Array|Add (Variables|Default|GetGridArray) _returnvalue))))

(fn GetClosestGridPosition
  (params (In%20Position :type Vector))
  (bind _output_get (LocalVariables|SetClosestPosition (Transformation|GetActorLocation (Utilities|Array|Get(acopy) (Variables|Default|GetGridArray)))))
  (LocalVariables|SetClosestDistance (Math|Vector|Distance(Vector) In%20Position _output_get))
  (for _array_element (Variables|Default|GetGridArray)
    (if (< (Math|Vector|Distance(Vector) (Transformation|GetActorLocation _array_element) In%20Position) (LocalVariables|GetClosestDistance))
      (LocalVariables|SetClosestPosition (Transformation|GetActorLocation _array_element))
      (LocalVariables|SetClosestDistance (Math|Vector|Distance(Vector) (Transformation|GetActorLocation _array_element) In%20Position))))
  (return (LocalVariables|GetClosestPosition)))