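; Cannon tower that repeatedly fires cannonballs for as long as it has a valid target.
; AttackSequence loops through Attack and a ShootDelay wait, with targeting state coming from outside this graph.
; Attack starts the firing montage and immediately spawns a BP_Cannon_Ball carrying Damage, at the barrel-socketed spawn point with TrackerComponent's rotation.
; Interface getters identify it as both cannon and tower.
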(event EventBeginPlay
  (|CallParentFunction))

(event Collision|EventActorBeginOverlap
  (params (OtherActor :type Actor%20Object%20Reference))
  (|CallParentFunction OtherActor) ; This node is disabled and will not be called.\nDrag off pins to build functionality.
)

(event EventTick
  (params (DeltaSeconds :type Float%20%28single-precision%29))
  (|CallParentFunction DeltaSeconds) ; This node is disabled and will not be called.\nDrag off pins to build functionality.
)

(event EventAttackSequence
  (params (Target :type Actor%20Object%20Reference))
  (if (Utilities|IsValid (Variables|Default|GetTarget)) :!label _label
    (CallFunction|Attack (Variables|Default|GetTarget))
    (Utilities|FlowControl|Delay (Variables|Default|GetShootDelay))
    (goto _label)))

(event EventAttack
  (params (Target :type Actor%20Object%20Reference))
  (Animation|Montage|PlayMontage (Variables|Default|GetSkeletalMesh) "/Game/Modelos_3D/Cañon/Animaciones/AM_CannonAttack.AM_CannonAttack"
    (:then
      (Game|SpawnActorfromClass "/Game/_Programacion/Angel/BP_Cannon_Ball.BP_Cannon_Ball_C" (Math|Transform|MakeTransform (Transformation|GetWorldLocation (Variables|Default|GetCannonball_Spawn)) (Transformation|GetWorldRotation (Variables|Default|GetTrackerComponent)) "1.000000,1.000000,1.000000") "Undefined" "MultiplyWithRoot" 0 (Variables|Default|GetDamage) 0))))

(fn ConstructionScript
  (|CallParentFunction)
  (Transformation|AttachComponentToComponent (Variables|Default|GetCannonball_Spawn) (Variables|Default|GetSkeletalMesh) "CannonBarrel" "SnapToTarget" "SnapToTarget" "KeepRelative" true))

(fn IGetSalamander
  (return 0))

(fn IGetCannon
  (return self))

(fn IGetTower
  (return self))