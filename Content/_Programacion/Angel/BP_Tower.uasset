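; Base tower Blueprint that detects, tracks and engages targets within a range sphere sized by Range in the Construction Script.
; Overlaps with BPI_Target actors maintain the Targets list; NewTarget picks the nearest on entry without a valid target, on any exit, or on OnKill.
; Tick turns the mesh toward the target while active and unbroken.
; NewTarget calls AttackSequence, which, like Attack, is an empty event here.
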(event OnComponentBeginOverlap(Sphere)
  (params (OverlappedComponent :type Primitive%20Component%20Object%20Reference) (OtherActor :type Actor%20Object%20Reference) (OtherComp :type Primitive%20Component%20Object%20Reference) (OtherBodyIndex :type Integer) (bFromSweep :type Boolean) (SweepResult :type Hit%20Result%20Structure%20%28by%20ref%29))
  (if (Utilities|DoesObjectImplementInterface OtherActor "/Game/_Programacion/Angel/Interface/BPI_Target.BPI_Target_C")
    (bind _selfactor (Class|BPITarget|IGetOwn(Message) OtherActor))
    (Utilities|Array|Add (Variables|Default|GetTargets) _selfactor)
    (Variables|Default|GetTarget
      (:then)
      (:else
        (CallFunction|NewTarget)))))

(event OnComponentEndOverlap(Sphere)
  (params (OverlappedComponent :type Primitive%20Component%20Object%20Reference) (OtherActor :type Actor%20Object%20Reference) (OtherComp :type Primitive%20Component%20Object%20Reference) (OtherBodyIndex :type Integer))
  (if (Utilities|DoesObjectImplementInterface OtherActor "/Game/_Programacion/Angel/Interface/BPI_Target.BPI_Target_C")
    (bind _selfactor (Class|BPITarget|IGetOwn(Message) OtherActor))
    (Utilities|Array|RemoveItem (Variables|Default|GetTargets) _selfactor)
    (CallFunction|NewTarget)))

(event Custom|Attack
  (params (Target :type Actor%20Object%20Reference)))

(event Custom|NewTarget
  (bind _targets (Variables|Default|GetTargets))
  (Variables|Default|SetTarget 0)
  (if (Utilities|Array|IsNotEmpty _targets)
    (Variables|Default|SetTarget (.ReturnValue (Actor|FindNearestActor (Transformation|GetActorLocation self) _targets)))
    (Variables|Default|SetActive true)
    (CallFunction|AttackSequence (Variables|Default|GetTarget))
    (else
      (Variables|Default|SetActive false))))

(event Custom|OnKill
  (Variables|Default|SetActive false)
  (CallFunction|NewTarget))

(event Custom|AttackSequence
  (params (Target :type Actor%20Object%20Reference)))

(event EventBeginPlay)

(event Collision|EventActorBeginOverlap
  (params (OtherActor :type Actor%20Object%20Reference)))

(event EventTick
  (params (DeltaSeconds :type Float%20%28single-precision%29))
  (if (and (Variables|Default|GetActive) (not (Variables|Default|GetBroken)))
    (Transformation|SetWorldRotation (Variables|Default|GetStaticMesh) (Math|Rotator|FindLookatRotation (Transformation|GetActorLocation self) (Transformation|GetActorLocation (Variables|Default|GetTarget))) false false)))

(fn ConstructionScript
  (Components|Sphere|SetSphereRadius (Variables|Default|GetSphere) (Variables|Stats|GetRange) false))