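; BP_Salamander is a salamander attacker Blueprint that repeatedly attacks its target and carries a Niagara fire effect.
; AttackSequence loops while Target is valid, calling Attack on it and then waiting ShootDelay before checking again.
; The Attack event here only plays the salamander attack montage on the skeletal mesh.
; The construction script runs the parent's, then attaches the fire system to the mesh's head socket.
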(event EventBeginPlay
  (|CallParentFunction) ; This node is disabled and will not be called.\nDrag off pins to build functionality.
)

(event Collision|EventActorBeginOverlap
  (params (OtherActor :type Actor%20Object%20Reference))
  (|CallParentFunction OtherActor) ; This node is disabled and will not be called.\nDrag off pins to build functionality.
)

(event EventTick
  (params (DeltaSeconds :type Float%20%28single-precision%29))
  (|CallParentFunction DeltaSeconds) ; This node is disabled and will not be called.\nDrag off pins to build functionality.
)

(event EventAttackSequence
  (params (Target :type Actor%20Object%20Reference))
  (if (Utilities|IsValid (Variables|Default|GetTarget)) :!label _label
    (CallFunction|Attack (Variables|Default|GetTarget))
    (Utilities|FlowControl|Delay (Variables|Default|GetShootDelay))
    (goto _label)))

(event EventAttack
  (params (Target :type Actor%20Object%20Reference))
  (Animation|Montage|PlayMontage (Variables|Default|GetSkeletalMesh) "/Game/Modelos_3D/Salamandra/Animaciones/AM_SalamanderAttack.AM_SalamanderAttack"))

(fn ConstructionScript
  (|CallParentFunction)
  (Transformation|AttachComponentToComponent (Variables|Default|GetNiagaraFireSistem) (Variables|Default|GetSkeletalMesh) "CabezaSocket" "KeepRelative" "KeepRelative" "KeepRelative" true))