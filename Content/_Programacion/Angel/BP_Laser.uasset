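; BP_Laser is a laser tower that fires a Niagara beam, attached to a mesh socket, at its target.
; Unless broken on start, AttackSequence repeats attacks with a delay while the target stays valid.
; Each attack plays a montage and runs a timed tick loop of rising damage, calling OnKill if the target becomes invalid.
; Tick keeps the beam end on the target, and I_GetTower returns the actor itself.
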(event EventBeginPlay
  (|CallParentFunction) ; This node is disabled and will not be called.\nDrag off pins to build functionality.
)

(event Collision|EventActorBeginOverlap
  (params (OtherActor :type Actor%20Object%20Reference))
  (|CallParentFunction OtherActor) ; This node is disabled and will not be called.\nDrag off pins to build functionality.
)

(event EventTick
  (params (DeltaSeconds :type Float%20%28single-precision%29))
  (|CallParentFunction DeltaSeconds)
  (if (Variables|Default|GetAttacking)
    (bind _target (Variables|Default|GetTarget)
      (:then
        (Niagara|SetNiagaraVariable(Vector3) (Variables|Default|GetNiagaraLaser) "Beam End" (Transformation|GetActorLocation _target)))
      (:else))))

(event EventAttackSequence
  (params (Target :type Actor%20Object%20Reference))
  (if (not (Variables|Default|GetBroken))
    (if (Utilities|IsValid (Variables|Default|GetTarget)) :!label _label
      (CallFunction|Attack (Variables|Default|GetTarget))
      (Utilities|FlowControl|Delay (Variables|Default|GetShootDelay))
      (goto _label))))

(event EventAttack
  (params (Target :type Actor%20Object%20Reference))
  (bind _niagaralaser (Variables|Default|GetNiagaraLaser))
  (Animation|Montage|PlayMontage (Variables|Default|GetSkeletalMesh) "/Game/Modelos_3D/Torre_Magica/Animacion/AM_GemAttack.AM_GemAttack"
    (:then
      (Variables|Default|SetAttacking true)
      (Components|Activation|Activate _niagaralaser true)
      (Variables|Default|SetLaserTickCount 1)
      (bind _target (Variables|Default|GetTarget :!label _label)
        (:then
          (Game|Damage|ApplyDamage _target (* (Variables|Default|GetDamage) (Variables|Default|GetLaserTickCount)) 0 self "/Game/_Programacion/Angel/Interface/DamageType_Enemy.DamageType_Enemy_C")
          (bind _result (Math|Integer|IncrementInt (Variables|Default|GetLaserTickCount))
            (:%20%20
              (if (> _result 10)
                _
                (else
                  (Utilities|FlowControl|Delay 0.1)
                  (goto _label))))))
        (:else
          (CallFunction|OnKill)))
      (Components|Activation|Deactivate _niagaralaser)
      (Variables|Default|SetAttacking false))))

(fn ConstructionScript
  (|CallParentFunction)
  (Transformation|AttachComponentToComponent (Variables|Default|GetNiagaraLaser) (Variables|Default|GetSkeletalMesh) "RaySocket" "SnapToTarget" "SnapToTarget" "KeepRelative" true))

(fn IGetTower
  (return self))