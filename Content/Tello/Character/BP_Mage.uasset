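; BP_Mage is a mage character that plays attack animations against towers and removes itself when it dies.
; Tick polls the CBPHealt component and, at zero health or below, plays the death montage once, then destroys the actor after a delay.
; Capsule overlap with an actor tagged "tower" starts a delayed loop replaying the attack montage, with no overlap-end or health check.
; No damage is applied in this graph.
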(event OnComponentBeginOverlap(CapsuleComponent)
  (params (OverlappedComponent :type Primitive%20Component%20Object%20Reference) (OtherActor :type Actor%20Object%20Reference) (OtherComp :type Primitive%20Component%20Object%20Reference) (OtherBodyIndex :type Integer) (bFromSweep :type Boolean) (SweepResult :type Hit%20Result%20Structure%20%28by%20ref%29))
  (if (Actor|ActorHasTag OtherActor "tower") :!label _label
    (Animation|PlayAnimMontage "/Game/Tello/Character/Animations/AM_Actions.AM_Actions" 1.0 "AttackMage")
    (Utilities|FlowControl|Delay 3.0)
    (goto _label)))

(event EventBeginPlay
  (|CallParentFunction) ; This node is disabled and will not be called.\nDrag off pins to build functionality.
)

(event Collision|EventActorBeginOverlap
  (params (OtherActor :type Actor%20Object%20Reference))
  (|CallParentFunction OtherActor) ; This node is disabled and will not be called.\nDrag off pins to build functionality.
)

(event EventTick
  (params (DeltaSeconds :type Float%20%28single-precision%29))
  (if (<= (Variables|/Game/Tello/Character/CBP_HealtTroops.CBP_HealtTroops_C|GetHealt (Variables|Default|GetCBP_Healt)) 0.0)
    (Utilities|FlowControl|DoOnce false
      (:Completed
        (Animation|PlayAnimMontage "/Game/Tello/Character/Animations/AM_Deaths.AM_Deaths" 1.0 "DeathMage")
        (Utilities|FlowControl|Delay 4.2)
        (Actor|DestroyActor)))))

(fn ConstructionScript
  (|CallParentFunction))