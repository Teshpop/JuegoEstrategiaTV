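; BP_EnemyNPC is an enemy pawn that wanders the level and chases any pawn it sees.
; From BeginPlay it walks slowly to random reachable points, repeating after a short delay only when a move succeeds.
; PawnSensing raises its speed and starts an AIMoveTo toward the seen pawn.
; The attack montage plays as soon as that move is issued, without waiting for arrival.
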(event OnSeePawn(PawnSensing)
  (params (Pawn :type Pawn%20Object%20Reference))
  (Variables|/Script/Engine.CharacterMovementComponent|SetMaxWalkSpeed (Variables|Character|GetCharacterMovement) 4e+02)
  (AI|AIMoveTo self (.RandomLocation (AI|Navigation|GetRandomReachablePointinRadius (Transformation|GetActorLocation self) 0.0 0 0)) Pawn 5.0 false
    (:then
      (Animation|PlayAnimMontage "/Game/Felipe/Anims/animattack.animattack" 1.0 "None"))))

(event Custom|Roaming
  (Variables|/Script/Engine.CharacterMovementComponent|SetMaxWalkSpeed (Variables|Character|GetCharacterMovement) 1.5e+02)
  (AI|AIMoveTo self (.RandomLocation (AI|Navigation|GetRandomReachablePointinRadius (Transformation|GetWorldLocation (Variables|Character|GetMesh)) 1e+03 0 0)) 0 5.0 false
    (:OnSuccess
      (Utilities|FlowControl|Delay 0.2)
      (CallFunction|Roaming))))

(event EventBeginPlay
  (CallFunction|Roaming))

(fn ConstructionScript)